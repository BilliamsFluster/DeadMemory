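; VR player character that sets floor tracking with stereo on and switches TimeHandler_BP weather to raining while G is held, snowing on release.
; The construction script detaches the mesh so CalculateMovement can place a body beneath and offset from the headset camera.
; That function retargets past movement or yaw thresholds, otherwise lerps toward the target, and sets height for IK.
; Its only call is unwired, so body following never runs.
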(event `self.ReceiveBeginPlay`
  (`KismetSystemLibrary.ExecuteConsoleCommand` "stereo on" null)
  (`HeadMountedDisplayFunctionLibrary.SetTrackingOrigin` "Floor")
  (bind _returnvalue (`GameplayStatics.GetActorOfClass` "/Game/_Game/DayNightTime/TimeHandler_BP.TimeHandler_BP_C"))
  (set `self.TimeHandler` _returnvalue))

(event `self.ReceiveTick`
  (params (DeltaSeconds :type "Float (single-precision)")))

(event `Key|G`
  (params (Key :type "Key Structure"))
  (bind _timehandler (`self.TimeHandler`))
  (:`Pressed`
    (`TimeHandler.SetWeatherCycle` _timehandler "WC_Raining"))
  (:`Released`
    (`TimeHandler.SetWeatherCycle` _timehandler "WC_Snowing")))

(fn `CalculateMovement`
  (locals (CurrentCameraPosition :type "Transform Structure") (DistanceRotated :type "Float (double-precision)" :default 0.0) (DistanceMoved :type "Float (double-precision)" :default 0.0))
  (bind (_location _rotation) (`self.GetBodyOffset`))
  (bind _bodycurrentposition (`self.BodyCurrentPosition`))
  (bind _returnvalue (`SceneComponent.K2_GetComponentToWorld` (`self.Camera`)))
  (bind _output_get (set `local.CurrentCameraPosition` (`KismetMathLibrary.MakeTransform` (`KismetMathLibrary.MakeVector` (.x (.location _returnvalue)) (.y (.location _returnvalue))) (`KismetMathLibrary.MakeRotator` 0.0 0.0 (.yaw (.rotation _returnvalue))))))
  (bind _distancemoved (`self.GetDistanceMoved` (.x (.location _output_get)) (.y (.location _output_get))))
  (set `local.DistanceMoved` _distancemoved)
  (bind _distancerotated (`self.GetDistanceRotated` (.rotation _output_get)))
  (set `local.DistanceRotated` _distancerotated)
  (`|ExecutionSequence`
    (:`then_0`
      ;[1 1 1] If Threshold is met set new position otherwise lerp to position
      (if (or (> (`local.DistanceMoved`) (`self.MovementThreshold`)) (> (`local.DistanceRotated`) (`self.RotationThreshold`)))
        (set `self.BodyTargetPosition` (`KismetMathLibrary.MakeTransform` _location _rotation))
        (set `self.MovementDirection` (`self.GetDirection` (`local.CurrentCameraPosition`)))
        (set `self.LastCameraPosition` (`local.CurrentCameraPosition`))
        (set `self.MovementSpeed` (/ (/ (+ (`local.DistanceMoved`) (`local.DistanceRotated`)) 2000.0) (`GameplayStatics.GetWorldDeltaSeconds`)))
        (elif (== (`self.BodyCurrentPosition`) (`self.BodyTargetPosition`))
          (set `self.MovementSpeed` 0.0)
          (set `self.MovementDirection` 0.0)
          (set `self.Alpha` 0.0)
          (else
            (set `self.Alpha` (`KismetMathLibrary.FInterpTo` (`self.Alpha`) 1.0 (`GameplayStatics.GetWorldDeltaSeconds`) (`self.MovementSpeed`)))
            (bind _output_get_2 (set `self.BodyCurrentPosition` (`KismetMathLibrary.TLerp` (`self.BodyCurrentPosition`) (`self.BodyTargetPosition`) (`self.Alpha`))))
            (`SceneComponent.K2_SetWorldLocationAndRotation` (`self.Mesh`) (.location _output_get_2) (.rotation _output_get_2) false false)))))
    (:`then_1`
      ;[1 1 1] Set Z for IK
      (`SceneComponent.K2_SetWorldLocationAndRotation` (`self.Mesh`) (`KismetMathLibrary.MakeVector` (.x (.location _bodycurrentposition)) (.y (.location _bodycurrentposition)) (.z (`self.GetBodyOffset`))) (.rotation _bodycurrentposition) false false))))

(fn `GetBodyOffset`
  (returns (Location :type "Vector Structure") (Rotation :type "Rotator Structure"))
  (bind _returnvalue (`SceneComponent.K2_GetComponentToWorld` (`self.Camera`)))
  (bind _returnvalue_2 (`KismetMathLibrary.MakeRotator` (.roll (.rotation _returnvalue)) (.pitch (.rotation _returnvalue)) (- (.yaw (.rotation _returnvalue)) 90.0)))
  (bind (_returnvalue_x _returnvalue_y _returnvalue_z) (`KismetMathLibrary.BreakVector` (+ (.location _returnvalue) (* (`KismetMathLibrary.GetRightVector` _returnvalue_2) -20))))
  (return (`KismetMathLibrary.MakeVector` _returnvalue_x _returnvalue_y (- _returnvalue_z (`self.PlayerHeight`))) _returnvalue_2))

(fn `GetBodyRotationFromHMD`
  (returns (Rotation :type "Rotator Structure"))
  (return (`KismetMathLibrary.MakeRotator` 0.0 0.0 (- (.yaw (.rotation (`SceneComponent.K2_GetComponentToWorld` (`self.Camera`)))) 90.0))))

(fn `GetDistanceMoved`
  (params (CurrentX :type "Float (double-precision)") (CurrentY :type "Float (double-precision)"))
  (returns (DistanceMoved :type "Float (double-precision)"))
  (bind _lastcameraposition (`self.LastCameraPosition`))
  (return (`KismetMathLibrary.Vector_Distance` (`KismetMathLibrary.MakeVector` CurrentX CurrentY) (`KismetMathLibrary.MakeVector` (.x (.location _lastcameraposition)) (.y (.location _lastcameraposition))))))

(fn `GetDistanceRotated`
  (params (CurrentRotation :type "Rotator Structure"))
  (returns (DistanceRotated :type "Float (double-precision)"))
  (return (`KismetMathLibrary.Abs` (- CurrentRotation_Yaw (.yaw (.rotation (`self.LastCameraPosition`)))))))

(fn `UserConstructionScript`
  (`SceneComponent.K2_DetachFromComponent` (`self.Mesh`) "KeepRelative" "KeepRelative" "KeepRelative" true))